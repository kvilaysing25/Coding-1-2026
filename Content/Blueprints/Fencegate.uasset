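; Fencegate is a toll gate that blocks entry to the garden until the player pays with a key, which the on-screen hint calls a coin.
; On overlap with BP_ThirdPersonCharacter it prints the toll message and checks that character's TotalKeys.
; With at least one key, it decrements the count and destroys the fence plank and overlap box components, opening the gate permanently; otherwise it prints a hint.
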(event EventBeginPlay)

(event Collision|EventActorBeginOverlap
  (params (OtherActor :type Actor%20Object%20Reference))
  (bind _asbp_third_person_character (Utilities|Casting|CastToBP_ThirdPersonCharacter OtherActor))
  (Development|PrintText "Only Those Willing to Pay May Enter The Garden")
  (if (> (Variables|/Game/ThirdPerson/Blueprints/BP_ThirdPersonCharacter.BP_ThirdPersonCharacter_C|GetTotal%20keys _asbp_third_person_character) 0)
    (Math|Integer|DecrementInt (Variables|/Game/ThirdPerson/Blueprints/BP_ThirdPersonCharacter.BP_ThirdPersonCharacter_C|GetTotal%20keys _asbp_third_person_character)
      (:%20%20
        (Components|DestroyComponent (Variables|Default|GetEA03_Fence_Plank_02d))
        (Components|DestroyComponent (Variables|Default|GetOverlap%20Box))))
    (else
      (Development|PrintText "Find a coin"))))

(event EventTick
  (params (DeltaSeconds :type Float%20%28single-precision%29)))

(fn ConstructionScript)
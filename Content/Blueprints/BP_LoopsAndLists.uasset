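; BP_LoopsAndLists is a demo Blueprint of loop and array techniques that randomly rotates BP_Tree actors.
; BeginPlay starts SimpleLoop, a Delay-driven endless loop calling LoopArrayOverTime every three seconds.
; That event shuffles the trees and steps through them with a counter and short Delay, setting random yaws.
; Uncalled examples show an all-at-once ForEach rotation and a While countdown printing in cycling colors.
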(event Custom|Simple%20Loop
  (Development|PrintText "Inside simple loop, waiting 3 seconds" :!label _label)
  (CallFunction|LoopArrayOverTime)
  (Utilities|FlowControl|Delay 3.0)
  (goto _label))

(event Custom|WhileLoop%20Function
  (bind _colors (Variables|Default|GetColors))
  (while (> (Variables|Default|GetWhileCounter) 0) ; If condition is true, keep looping
    (Development|PrintText (Utilities|Text|FormatText "This is loop {count}. Ran after {seconds} seconds." (Variables|Default|GetWhileCounter) (Utilities|Text|ToText(Float) (Utilities|Time|GetRealTimeSeconds) "HalfToEven" false true 1 324 3)) true true (Utilities|Array|Get(acopy) _colors (Math|Integer|%(Integer) (Variables|Default|GetWhileCounter) (Utilities|Array|Length _colors))) 2e+01)
    (Math|Integer|DecrementInt (Variables|Default|GetWhileCounter))))

(event Custom|ChangeTreesForEach
  (bind _outactors (Actor|GetAllActorsOfClass "/Game/Blueprints/BP_Tree.BP_Tree_C"))
  (for _array_element _outactors
    (Transformation|SetActorRelativeRotation _array_element (Math|Rotator|MakeRotator 0.0 0.0 (Math|Random|RandomFloatinRange 0.0 3.6e+02))))
  (Development|PrintText "Trees have been rotated"))

(event Custom|Loop%20Array%20Over%20Time
  (bind _outactors (Actor|GetAllActorsOfClass "/Game/Blueprints/BP_Tree.BP_Tree_C"))
  (Utilities|Array|Shuffle _outactors)
  (if (< (Variables|Default|GetOverTimeIndex) (Utilities|Array|Length _outactors)) :!label _label ; test for the loop
    (Transformation|SetActorRelativeRotation (Utilities|Array|Get(acopy) _outactors (Variables|Default|GetOverTimeIndex)) (Math|Rotator|MakeRotator 0.0 0.0 (Math|Random|RandomFloatinRange 0.0 3.6e+02)))
    (Math|Integer|IncrementInt (Variables|Default|GetOverTimeIndex)
      (:%20%20
        (Utilities|FlowControl|Delay 0.2)
        (goto _label)))
    (else
      (Variables|Default|SetOverTimeIndex 0) ; reset index to zero
    )))

(event EventBeginPlay
  (Development|PrintText "Loops and lists is Starting")
  (CallFunction|SimpleLoop))

(fn ConstructionScript)